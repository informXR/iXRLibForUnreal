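; BP_LevelManager is a level actor that starts the IXR library on BeginPlay and sets up the startup UI for the current platform.
; On Android it toggles on the VRPawn menu; on other platforms it adds a WBP_Keyboard widget to the viewport.
; Codes submitted through that keyboard go to KeyboardAuthenticate, with the result reported only by placeholder debug prints.
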(event `self.ReceiveBeginPlay`
  (`IXRBlueprintLibrary.StartIXRLib_BFL`)
  (if (`KismetStringLibrary.EqualEqual_StrStr` "Android" (`GameplayStatics.GetPlatformName`))
    (bind _asvrpawn (cast `/IXRLib/VRTemplate/Blueprints/VRPawn` (`GameplayStatics.GetPlayerPawn` 0)))
    (`/IXRLib/VRTemplate/Blueprints/VRPawn.ToggleMenu` _asvrpawn true)
    (else
      (bind _returnvalue (`|CreateWidget` "/IXRLib/UI/WBP_Keyboard.WBP_Keyboard_C" (`GameplayStatics.GetPlayerController` 0)))
      (`UserWidget.AddToViewport` _returnvalue 0)
      (add `/IXRLib/UI/WBP_Keyboard.OnSubmitCodeEvent` _returnvalue (delegate `OnSubmitCodeEvent_Event`)))))

(event `OnSubmitCodeEvent_Event`
  (params (InputCode :type String))
  (bind _returnvalue (`IXRBlueprintLibrary.KeyboardAuthenticate` InputCode))
  (if _returnvalue
    (`KismetSystemLibrary.PrintString` "Hello")
    (else
      (`KismetSystemLibrary.PrintString` "rerere"))))

(fn `UserConstructionScript`)